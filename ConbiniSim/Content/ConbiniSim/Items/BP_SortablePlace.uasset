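; BP_SortablePlace is a storage spot in the convenience store sim that the player stocks from a held or targeted BP_Package.
; GiveAction accepts an item while space remains and its name matches the stored type, or no type is set.
; It finds the item's DT_Item row, spawns that actor on the next of ten scene slots without physics or collision, and decrements the package amount.
; Both grabbing functions return false.
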(event `/Game/ConbiniSim/Items/BPI_Interactable.GiveAction`
  (bind _name (break `/Game/ConbiniSim/Items/S_Item` (`self.StorageItemInfo`)))
  (bind _returnvalue (select `int` (`self.CurrentAmount`) :`0` (`self.Scene`) :`1` (`self.Scene1`) :`2` (`self.Scene2`) :`3` (`self.Scene3`) :`4` (`self.Scene4`) :`5` (`self.Scene5`) :`6` (`self.Scene6`) :`7` (`self.Scene7`) :`8` (`self.Scene8`) :`9` (`self.Scene9`)))
  (bind _asbp_first_person_character (cast `/Game/FirstPerson/Blueprints/BP_FirstPersonCharacter` (`GameplayStatics.GetPlayerCharacter` 0)))
  (bind _asbp_package (cast `/Game/ConbiniSim/Items/BP_Package` (`/Game/FirstPerson/Blueprints/BP_FirstPersonCharacter.InteractableActor` _asbp_first_person_character)))
  (bind _item (`/Game/ConbiniSim/Items/BP_Package.Item` _asbp_package))
  (bind (_itemtobuy _amount) (break `/Game/ConbiniSim/Main/S_BuyingItems` _item))
  (if (and (< (`self.CurrentAmount`) (`self.AmountPerStorage`)) (or (`KismetTextLibrary.EqualEqual_TextText` (`.Name_2_6CB8791A482D6092D41BD58E6FF575B0` (break `/Game/ConbiniSim/Items/S_Item` _itemtobuy)) _name) (`KismetTextLibrary.TextIsEmpty` _name)))
    (bind _output_get (set `self.StorageItemInfo` _itemtobuy))
    (bind _outrownames (`DataTableFunctionLibrary.GetDataTableRowNames` "/Game/ConbiniSim/Items/DT_Item.DT_Item"))
    (for _array_element _outrownames
      (bind _returnvalue_2 (`|GetDataTableRow` "/Game/ConbiniSim/Items/DT_Item.DT_Item" _array_element)
        (:`then`
          (bind (_name_2 _description _unitamount _thumbnail _actor) (break `/Game/ConbiniSim/Items/S_Item` _returnvalue_2))
          (if (`KismetTextLibrary.EqualEqual_TextText` _name_2 (`.Name_2_6CB8791A482D6092D41BD58E6FF575B0` (break `/Game/ConbiniSim/Items/S_Item` _output_get)))
            (bind _returnvalue_3 (`|SpawnActorFromClass` _actor (`KismetMathLibrary.MakeTransform` (`SceneComponent.K2_GetComponentLocation` _returnvalue)) "Undefined" "MultiplyWithRoot" null (make `DataTableRowHandle` "/Game/ConbiniSim/Items/DT_Item.DT_Item" _array_element) null))
            (bind _itemmesh (`/Game/ConbiniSim/Items/BP_Item.ItemMesh` _returnvalue_3))
            (`PrimitiveComponent.SetCollisionEnabled` _itemmesh "NoCollision")
            (`self.K2_AttachToComponent` _returnvalue_3 _returnvalue "None" "SnapToTarget" "SnapToTarget" "SnapToTarget" true)
            (`PrimitiveComponent.SetSimulatePhysics` _itemmesh false)
            (`/Engine/EditorBlueprintResources/StandardMacros.IncrementInt` (`self.CurrentAmount`))))))
    (setmembers `/Game/ConbiniSim/Main/S_BuyingItems` :`StructRef` _item :`Amount` (- _amount 1))))

(fn `RemoveGrabbing`
  (returns (Sucess :type Boolean))
  (return false))

(fn `StartGrabbing`
  (returns (Sucess :type Boolean))
  (return false))

(fn `UserConstructionScript`)