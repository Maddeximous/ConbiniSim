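; BP_Simulator_PC is the player controller for the ConbiniSim game, owning the player HUD and pricing the items being bought.
; On BeginPlay, the local controller creates WBP_PlayerHUD and adds it to the viewport.
; CalculateTotal sums price times amount across BuyingItems.
; ToggleHUD_1 sets the HUD to Visible whatever ShouldShow is, and GetMainController has an empty return.
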(event `self.ReceiveBeginPlay`
  (if (`self.IsLocalPlayerController`)
    ; Create Player HUD Widget
    (bind _returnvalue (`|CreateWidget` "/Game/ConbiniSim/UI/WBP_PlayerHUD.WBP_PlayerHUD_C"))
    (bind _output_get (set `self.PlayerHud` _returnvalue))
    (`UserWidget.AddToViewport` _output_get 0)))

(event `ToggleHUD_1`
  (params (ShouldShow :type Boolean))
  (`Widget.SetVisibility` (`self.PlayerHud`) (select `bool` ShouldShow :`false` "Visible" :`true` "Visible" :!type "ESlateVisibility Enum")))

(fn `CalculateTotal`
  (returns (TotalPrice :type "Float (double-precision)"))
  (locals (LocalTotalPrice :type "Float (double-precision)"))
  (for _array_element (`self.BuyingItems`)
    (bind (_itemtobuy _amount) (break `/Game/ConbiniSim/Main/S_BuyingItems` _array_element))
    (set `local.LocalTotalPrice` (+ (* (`.Price_7_6113806E4FB3CC1A0D7E79B1E7F98F50` (break `/Game/ConbiniSim/Items/S_Item` _itemtobuy)) _amount) (`local.LocalTotalPrice`))))
  (return (`local.LocalTotalPrice`)))

(fn `GetMainController`
  (returns (PC_Ref :type "/Game/ConbiniSim/Main/BP_Simulator_PC Object Reference"))
  (return null))

(fn `UserConstructionScript`)