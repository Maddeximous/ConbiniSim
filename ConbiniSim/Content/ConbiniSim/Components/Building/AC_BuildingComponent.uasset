(event `self.ReceiveTick`
  (params (DeltaSeconds :type "Float (single-precision)"))
  ; Loop for Building
  (if (`self.bInBuildMode`)
    (`self.PreviewLoop`)))

(event `self.ReceiveBeginPlay`
  (bind _asbp_first_person_character (cast `/Game/FirstPerson/Blueprints/BP_FirstPersonCharacter` (`self.GetOwner`)))
  (set `self.PlayerRef` _asbp_first_person_character)
  (set `self.CameraRef` (`ConbiniSimCharacter.FirstPersonCameraComponent` _asbp_first_person_character)))

(event `ResetBuildMode`
  (goto _label :!via `Reset`))

(event `PreviewLoop`
  (bind _cameraref (`self.CameraRef`))
  (bind _returnvalue (`SceneComponent.K2_GetComponentLocation` _cameraref))
  (bind _returnvalue_2 (`SceneComponent.GetForwardVector` _cameraref))
  (bind (_outhit _returnvalue_3) (`KismetSystemLibrary.LineTraceSingle` (+ _returnvalue (* _returnvalue_2 350.0)) (+ _returnvalue (* _returnvalue_2 1000.0)) "TraceTypeQuery1" false (`|MakeArray` (`self.GetOwner`)) "ForOneFrame"))
  (if _returnvalue_3
    (`|ExecutionSequence`
      (:`then_0`
        (`/Engine/EditorBlueprintResources/StandardMacros.DoOnce` false :!label _label
          (:`Completed`
            (bind _returnvalue_4 (`|AddComponentByClass` (`self.PlayerRef`) "/Script/Engine.StaticMeshComponent" false (`self.BuildTransform`)))
            ; Set Preview mesh for Building
            (bind _output_get (set `self.PreviewMesh` _returnvalue_4))
            (bind _returnvalue_5 (`|GetDataTableRow` "/Game/ConbiniSim/Items/DT_Item.DT_Item" (`.RowName` (break `DataTableRowHandle` (`/Game/ConbiniSim/Items/BP_Item.ItemRef` (`self.InteractActor`)))))
              (:`then`
                (`StaticMeshComponent.SetStaticMesh` _output_get (`.PreviewMesh_30_004ADE434B942065C571B5B2690C717E` (break `/Game/ConbiniSim/Items/S_Item` _returnvalue_5)))
                (`PrimitiveComponent.SetMaterial` _output_get 0 "/Game/ConbiniSim/Materials/M_BuildingPreview.M_BuildingPreview")
                (`PrimitiveComponent.SetCollisionEnabled` (`self.PreviewMesh`) "NoCollision"))))))
      (:`then_1`
        (set `self.BuildTransform` (`KismetMathLibrary.MakeTransform` (`.Location` (`GameplayStatics.BreakHitResult` _outhit))))
        (`SceneComponent.K2_SetWorldTransform` (`self.PreviewMesh`) (`self.BuildTransform`) false false)))))

(event `SHouldActivateBuildMode`
  (params (InteractActor :type "/Game/ConbiniSim/Items/BP_Item Object Reference"))
  (if (not (`self.bInBuildMode`))
    (set `self.bInBuildMode` true)
    (set `self.InteractActor` InteractActor)
    (else
      (set `self.bInBuildMode` false :!label _label_2)
      (set `self.InteractActor` null)
      (`self.ResetBuildMode`)
      (message `/Game/ConbiniSim/PBI_PlayerInterface.DestoryComponent` (`self.GetOwner`) (`self.PreviewMesh`))
      (set `self.PreviewMesh` null))))

(event `StopBuildMode`
  (goto _label_2))

(event `Build`
  (if (`self.bInBuildMode`)
    (`|SpawnActorFromClass` "/Game/ConbiniSim/Items/BP_Shelf.BP_Shelf_C" (`self.BuildTransform`) "AdjustIfPossibleButAlwaysSpawn" "MultiplyWithRoot" null (struct) null)
    (`self.StopBuildMode`)))